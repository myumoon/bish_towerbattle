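; Background actor that follows the GameCamera and shifts its color when game over starts.
; Each tick it moves by the camera's position change since the last frame, keeping its offset from the camera.
; StartGameOver starts a timed lerp of hue offset and value parameters on a dynamic material instance created in the Construction Script, running from 1.0 to configured end values.
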(event `self.ReceiveBeginPlay`
  (set `self.PrevCameraPos` (`self.K2_GetActorLocation` (`/Game/NkLib/NkUtil.GetActorOfClass` "/Game/System/GameCamera.GameCamera_C"))))

(event `self.ReceiveTick`
  (params (DeltaSeconds :type "Float (single-precision)"))
  (bind _returnvalue (`self.K2_GetActorLocation` (`/Game/NkLib/NkUtil.GetActorOfClass` "/Game/System/GameCamera.GameCamera_C")))
  (`|ExecutionSequence`
    (:`then_0`
      (if (`self.StartedColorChange`)
        (bind _output_get (set `self.CurrentChangeSec` (+ DeltaSeconds (`self.CurrentChangeSec`))))
        (bind _returnvalue_2 (`KismetMathLibrary.FClamp` (/ _output_get (`self.HueChangeSec`))))
        (`MaterialInstanceDynamic.SetScalarParameterValue` (`self.Material`) "HueOffsetPercent" (`KismetMathLibrary.Lerp` 1.0 (`self.EndHueOffsetPercent`) _returnvalue_2))
        (`MaterialInstanceDynamic.SetScalarParameterValue` (`self.Material`) "ValuePercent" (`KismetMathLibrary.Lerp` 1.0 (`self.EndValuePercent`) _returnvalue_2))
        (if (>= (`self.CurrentChangeSec`) (`self.HueChangeSec`))
          (set `self.StartedColorChange` false))))
    (:`then_1`
      (`self.K2_AddActorWorldOffset` (- _returnvalue (`self.PrevCameraPos`)))
      (set `self.PrevCameraPos` _returnvalue))))

(fn `StartGameOver`
  (set `self.CurrentChangeSec` 0.0)
  (set `self.StartedColorChange` true))

(fn `UserConstructionScript`
  (bind _returnvalue (`PrimitiveComponent.CreateDynamicMaterialInstance` (`self.StaticMeshComponent`) 0 "/Game/BG/Textures/bg_Mat.bg_Mat"))
  (set `self.Material` _returnvalue))