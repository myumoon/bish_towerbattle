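; Background moon Blueprint whose emissive glow brightens while the player touches it and fades back after release.
; The construction script creates a dynamic material from MoonMat on the static mesh.
; Touch begin, end and leave events toggle a flag that Tick uses to ramp a clamped alpha up or down over time.
; UpdateMaterial runs every Tick, adding the ease-in enhancement to base emissive strength and applying shadow strength.
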(event `self.ReceiveBeginPlay`)

(event `self.ReceiveTick`
  (params (DeltaSeconds :type "Float (single-precision)"))
  (`|ExecutionSequence`
    (:`then_0`
      (if (`self.IsTouched`)
        (set `self.EmissiveEnhanceAlpha` (`KismetMathLibrary.FMin` (+ (`self.EmissiveEnhanceAlpha`) (* (`self.EmissiveAlphaPerSec`) DeltaSeconds)) 1.0))
        (else
          (set `self.EmissiveEnhanceAlpha` (`KismetMathLibrary.FMax` (- (`self.EmissiveEnhanceAlpha`) (* (`self.EmissiveAlphaPerSec`) DeltaSeconds)))))))
    (:`then_1`
      (`self.UpdateMaterial`))))

(event `self.StaticMeshComponent.OnInputTouchBegin`
  (params (FingerIndex :type "ETouchIndex Enum" :default "Touch1") (TouchedComponent :type "PrimitiveComponent Object Reference"))
  (set `self.IsTouched` true))

(event `self.StaticMeshComponent.OnInputTouchEnd`
  (params (FingerIndex :type "ETouchIndex Enum" :default "Touch1") (TouchedComponent :type "PrimitiveComponent Object Reference"))
  (set `self.IsTouched` false :!label _label))

(event `self.StaticMeshComponent.OnInputTouchLeave`
  (params (FingerIndex :type "ETouchIndex Enum" :default "Touch1") (TouchedComponent :type "PrimitiveComponent Object Reference"))
  (goto _label))

(fn `UpdateMaterial`
  (`MaterialInstanceDynamic.SetScalarParameterValue` (`self.Material`) "EmissiveStrength" (+ (`|EaseFunction` "EaseIn" (`self.EmissiveEnhanceAlpha`) 0.0 (`self.MaxEmissiveEnhance`)) (`self.EmissiveStrength`)))
  (`MaterialInstanceDynamic.SetScalarParameterValue` (`self.Material`) "ShadowStrength" (`self.ShadowStrength`)))

(fn `UserConstructionScript`
  (bind _returnvalue (`PrimitiveComponent.CreateDynamicMaterialInstance` (`self.StaticMeshComponent`) 0 "/Game/BG/Materials/MoonMat.MoonMat"))
  (set `self.Material` _returnvalue))