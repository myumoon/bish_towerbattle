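; A Paper2D block actor that the player rotates, positions and drops, driven by a state machine on Tick.
; Initialize registers it with the GameManager and sets its sprite, then a timeline scales it up into Rotation state.
; InputManager drag eases the sprite toward the next table angle and snaps at a threshold; touching the block switches to Movement.
; Movement follows the fall position until release enables physics, where time spent stable is accumulated.
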(event `OnSpawn`
  (bind _finalscale (`self.FinalScale`))
  (bind (_direction _scale) (`Timeline|ScaleTimeline` :!via `PlayFromStart`)
    (:`Update`
      (`SceneComponent.SetWorldScale3D` (`self.PaperSprite`) (* (`KismetMathLibrary.MakeVector` _finalscale 1.0 _finalscale) _scale)))
    (:`Finished`
      (`self.OnRotate`))))

(event `OnRotate`
  (set `self.State` "NewEnumerator1"))

(event `self.ReceiveTick`
  (params (DeltaSeconds :type "Float (single-precision)"))
  (switch `/Game/Blocks/BlockState` (`self.State`)
    (:`NewEnumerator1`
      (`self.UpdateRotation`))
    (:`NewEnumerator2`
      (`self.UpdateMovement`))
    (:`NewEnumerator6`
      (`self.UpdatePhysics` DeltaSeconds))))

(event `OnMovement`
  (set `self.State` "NewEnumerator2"))

(event `OnFall`
  (set `self.State` "NewEnumerator3")
  (`PrimitiveComponent.SetSimulatePhysics` (`self.PaperSprite`) true)
  (`PrimitiveComponent.SetEnableGravity` (`self.PaperSprite`) true)
  (set `self.State` "NewEnumerator6"))

(event `OnPhysics`
  (set `self.State` "NewEnumerator6"))

(event `OnFixed`)

(event `self.PaperSprite.OnInputTouchBegin`
  (params (FingerIndex :type "ETouchIndex Enum" :default "Touch1") (TouchedComponent :type "PrimitiveComponent Object Reference"))
  ;[1 1 1] ブロックにタッチしたら移動に遷移
  (if (`|EnumEquality` (`self.State`) "NewEnumerator1")
    (`self.OnMovement`)))

(fn `GetState`
  (returns (NewParam :type "/Game/Blocks/BlockState Enum"))
  (return (`self.State`)))

(fn `Initialize`
  (params (Sprite :type "PaperSprite Object Reference") (Scale :type "Float (double-precision)") (Position :type "Vector Structure"))
  (bind _papersprite (`self.PaperSprite`))
  (set `self.FinalScale` Scale)
  (`/Game/System/GameManager.SetCurrentBlock` (`/Game/System/GameUtil.GetGameManager`) self)
  (`PrimitiveComponent.SetSimulatePhysics` (`self.PaperSprite`) false) ; 物理を無効にしないと移動してくれない
  (`self.SetActorHiddenInGame` false)
  (`self.K2_SetActorLocation` Position false true)
  (`PaperSpriteComponent.SetSprite` _papersprite Sprite)
  (`SceneComponent.SetWorldScale3D` _papersprite (`KismetMathLibrary.MakeVector` 0.0))
  (`self.OnSpawn`))

(fn `UpdateMovement`
  (`|ExecutionSequence`
    (:`then_0`
      (if (`/Game/System/InputManager.Released` (`/Game/System/GameUtil.GetInputManager`))
        (`self.OnFall`)
        (return)))
    (:`then_1`
      (`self.K2_SetActorLocation` (`/Game/System/InputManager.GetFallPos` (`/Game/System/GameUtil.GetInputManager`))))))

(fn `UpdatePhysics`
  (params (DeltaTime :type "Float (double-precision)"))
  (if (<= (`KismetMathLibrary.VSizeSquared` (- (`self.K2_GetActorLocation`) (`self.PrevPos`))) (* (`self.StableLength`) (`self.StableLength`)))
    (set `self.StableTime` (+ (`self.StableTime`) DeltaTime))
    (else
      (set `self.StableTime` 0.0))))

(fn `UpdateRotation`
  (locals (RotAmount :type "Float (double-precision)"))
  (bind _mng (`/Game/System/GameUtil.GetInputManager`))
  (bind _switchrotamount (`self.SwitchRotAmount`))
  (bind _rotangletbl (`self.RotAngleTbl`))
  (bind _rotindex (`self.RotIndex`))
  (bind _returnvalue (`KismetArrayLibrary.Array_Length` _rotangletbl))
  (`|ExecutionSequence`
    (:`then_0`
      (if (`/Game/System/InputManager.Pressed` _mng)
        (set `self.Rotating` true)
        (set `self.BasetRot` (`SceneComponent.K2_GetComponentRotation` (`self.PaperSprite`)))
        (set `self.CurrentRot` 0.0)))
    (:`then_1`
      (if (`/Game/System/InputManager.Released` _mng)
        (set `self.Rotating` false)
        (`SceneComponent.K2_SetWorldRotation` (`self.PaperSprite`) (`self.BasetRot`) false false)))
    (:`then_2`
      (if true
        (bind _rotreverseclockamount (`/Game/System/InputManager.ConsumeRotateAmount` (`/Game/System/GameUtil.GetInputManager`)))
        (if (or (> _rotreverseclockamount 0.0) (< _rotreverseclockamount 0.0))
          (bind _output_get (set `self.CurrentRot` (+ _rotreverseclockamount (`self.CurrentRot`))))
          (bind _returnvalue_2 (/ (`KismetMathLibrary.FMin` (`KismetMathLibrary.Abs` _output_get) _switchrotamount) _switchrotamount))
          (if (>= _returnvalue_2 1.0)
            ;[1 1 1] 一定距離動かしたらカクッって感じで一気に45度単位で進める
            (if (>= (`self.CurrentRot`) 0.0)
              (`/Engine/EditorBlueprintResources/StandardMacros.IncrementInt` _rotindex
                (:`  `
                  _))
              (else
                (`/Engine/EditorBlueprintResources/StandardMacros.DecrementInt` _rotindex
                  (:`  `
                    _))))
            (set `self.RotIndex` (mod (+ (`self.RotIndex`) _returnvalue) _returnvalue))
            (bind _output_get_2 (set `self.BasetRot` (`KismetMathLibrary.MakeRotator` 0.0 (`|GetArrayItem` _rotangletbl (`self.RotIndex`)))))
            (`SceneComponent.K2_SetWorldRotation` (`self.PaperSprite`) _output_get_2 false false)
            (set `self.CurrentRot` 0.0)
            (else
              ;[1 1 1] 動かし始めはゆっくり動いて、45度に近づくにつれて早く動かす
              (if (>= (`self.CurrentRot`) 0.0)
                (bind _returnvalue_3 (* 30.0 (`KismetMathLibrary.MultiplyMultiply_FloatFloat` _returnvalue_2 3.5)))
                (set `local.RotAmount` _returnvalue_3)
                (else
                  (set `local.RotAmount` (* _returnvalue_3 -1.0))))
              (`SceneComponent.K2_SetWorldRotation` (`self.PaperSprite`) (`KismetMathLibrary.MakeRotator` 0.0 (+ (`local.RotAmount`) (`|GetArrayItem` (`self.RotAngleTbl`) (`self.RotIndex`)))) false false))))))))

(fn `UserConstructionScript`
  (`PrimitiveComponent.SetEnableGravity` (`self.PaperSprite`) false))